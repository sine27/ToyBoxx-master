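; BP_Target_Wild is a lesson target that bursts in a small neon explosion and returns a fixed score-like value when Interact is called.
; On BeginPlay it stores its origin, waits a random few seconds, then plays the WindCurve timeline.
; Each timeline update sets its location to origin plus a vertical offset multiplied by a constant zero, so the target stays in place.
; Interact does not destroy or hide the actor.
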(event `self.ReceiveBeginPlay`
  (set `self.Origin` (`self.K2_GetActorLocation`))
  (`KismetSystemLibrary.Delay` (`KismetMathLibrary.RandomFloatInRange` 2.0 8.0))
  (`Timeline|WindCurve` :!via `PlayFromStart`
    (:`Update`
      (`self.K2_SetActorLocation` (+ (`self.Origin`) (* (0.0 0.0 100.0) 0.0))))))

(fn `Interact`
  (returns (Score :type Integer))
  (`GameplayStatics.SpawnEmitterAtLocation` "/Game/Effects/Particles/Explosion/P_NeonExplosion_Tiny.P_NeonExplosion_Tiny" (`self.K2_GetActorLocation`))
  (return 5))

(fn `UserConstructionScript`)