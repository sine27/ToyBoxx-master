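; BP_InteractionPlayer is a VR lesson player that interacts by gaze and scores hits on targets.
; Tick traces along the camera's forward vector and moves a billboard reticle to the hit point or the trace's far end.
; The Act input repeats that trace and calls Interact on a BP_InteractionTest or BP_Target.
; Target hits also increment Score, update the scoreboard found at BeginPlay and spawn a BP_ScoreAddition popup.
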(event `InputAction|Act`
  (params (Key :type "Key Structure" :default "AnyKey"))
  (:`Pressed`
    (bind (_location _forward_vector) (`/Game/Blueprints/Utility/LayoutVRUtilityFunctions.Get Player VR Camera Properties`))
    (bind (_outhit _returnvalue) (`KismetSystemLibrary.LineTraceSingle` _location (+ _location (* _forward_vector 10000)) "TraceTypeQuery1"))
    (if _returnvalue
      (bind (_bblockinghit _binitialoverlap _time _location_2 _impactpoint _normal _impactnormal _physmat _hitactor) (`GameplayStatics.BreakHitResult` _outhit))
      (bind _asbp_interaction_test (cast `/Game/Lessons/Lesson3/BP_InteractionTest` _hitactor)
        (:`then`
          (`/Game/Lessons/Lesson3/BP_InteractionTest.Interact` _asbp_interaction_test))
        (:`CastFailed`
          (bind _asbp_target (cast `/Game/Lessons/Lesson3/BP_Target` _hitactor))
          (`/Game/Lessons/Lesson3/BP_Target.Interact` _asbp_target)
          (bind _output_get (set `self.Score` (+ (`self.Score`) 1)))
          (`/Game/Lessons/Lesson3/BP_Scoreboard.UpdateScore` (`self.Scoreboard`) _output_get)
          (`|SpawnActorFromClass` "/Game/Lessons/Lesson3/BP_ScoreAddition.BP_ScoreAddition_C" (`KismetMathLibrary.MakeTransform` _location_2) "Undefined" "OverrideRootScale" null 1 20.0))))))

(event `self.ReceiveTick`
  (params (DeltaSeconds :type "Float (single-precision)"))
  (bind (_location _forward_vector) (`/Game/Blueprints/Utility/LayoutVRUtilityFunctions.Get Player VR Camera Properties`))
  (bind _returnvalue (+ _location (* _forward_vector 10000)))
  (bind (_outhit _returnvalue_2) (`KismetSystemLibrary.LineTraceSingle` _location _returnvalue "TraceTypeQuery1"))
  (if _returnvalue_2
    (`SceneComponent.K2_SetWorldLocation` (`self.MaterialBillboard`) (`.Location` (`GameplayStatics.BreakHitResult` _outhit)) false false)
    (else
      (`SceneComponent.K2_SetWorldLocation` (`self.MaterialBillboard`) _returnvalue false false))))

(event `self.ReceiveBeginPlay`
  (bind _outactors (`GameplayStatics.GetAllActorsOfClass` "/Game/Lessons/Lesson3/BP_Scoreboard.BP_Scoreboard_C"))
  (set `self.Scoreboard` (`KismetArrayLibrary.Array_Get` _outactors)))

(fn `UserConstructionScript`)