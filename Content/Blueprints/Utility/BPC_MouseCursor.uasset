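; Actor component that gives its owner a 3D mouse cursor by spawning a BP_MouseCursor actor at the owner's transform on BeginPlay.
; It acts as a facade over that actor, forwarding mouse deltas to its Update and returning the trace hit and result.
; Helper functions expose the cursor's world location and dynamic material, set its Color parameter, and toggle its in-game visibility.
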(event `self.ReceiveBeginPlay`
  (bind _returnvalue (`|SpawnActorFromClass` "/Game/Blueprints/Utility/BP_MouseCursor.BP_MouseCursor_C" (`Actor.GetTransform` (`self.GetOwner`)) "Undefined" "OverrideRootScale"))
  (set `self.Cursor` _returnvalue))

(fn `GetCursorDMI`
  (returns (CursorDMI :type "MaterialInstanceDynamic Object Reference"))
  (return (`/Game/Blueprints/Utility/BP_MouseCursor.CursorDMI` (`self.Cursor`))))

(fn `GetCursorLocation`
  (returns (CursorWorldLocation :type "Vector Structure"))
  (return (`SceneComponent.K2_GetComponentLocation` (`/Game/Blueprints/Utility/BP_MouseCursor.3DCursor` (`self.Cursor`)))))

(fn `SetCursorColor`
  (params (Color :type "LinearColor Structure"))
  (`MaterialInstanceDynamic.SetVectorParameterValue` (`/Game/Blueprints/Utility/BP_MouseCursor.CursorDMI` (`self.Cursor`)) "Color" Color))

(fn `SetCursorVisibility`
  (params (`New Visibility` :type Boolean))
  (`Actor.SetActorHiddenInGame` (`self.Cursor`) (not `New Visibility`)))

(fn `Update`
  (params (DeltaX :type "Float (double-precision)") (DeltaY :type "Float (double-precision)"))
  (returns (TraceHit :type "HitResult Structure") (TraceResult :type Boolean))
  (bind (_tracehit _traceresult) (`/Game/Blueprints/Utility/BP_MouseCursor.Update` (`self.Cursor`) DeltaX DeltaY))
  (return _tracehit _traceresult))